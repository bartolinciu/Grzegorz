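; AI black hole pawn that chases the player, pulls them in and hurts them up close.
; Each Tick issues an AI MoveTo toward the player character with a wide acceptance radius.
; On success, a small additive LaunchCharacter nudges the player opposite the hole's view direction, drawing them in when it faces them.
; The same success path applies light damage when the player is very near its center.
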(event EventBeginPlay)

(event Collision|EventActorBeginOverlap
  (params (OtherActor :type Actor%20Object%20Reference)))

(event EventTick
  (params (DeltaSeconds :type Float%20%28single-precision%29))
  (bind _returnvalue (Game|GetPlayerCharacter 0))
  (AI|AIMoveTo self "0, 0, 0" _returnvalue 8e+02 false
    (:OnSuccess
      (Character|LaunchCharacter _returnvalue (* (Math|Vector|GetForwardVector (.OutRotation (Actor|GetActorEyesViewPoint))) "-5.000000,-5.000000,-5.000000") false false)
      (Math|Float|CompareFloat (Math|Vector|Distance(Vector) (Transformation|GetActorLocation) (Transformation|GetActorLocation _returnvalue)) 1e+02
        (:<
          (Game|Damage|ApplyDamage _returnvalue 1.0 0 0))))))

(fn ConstructionScript)